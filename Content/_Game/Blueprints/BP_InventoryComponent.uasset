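; Inventory slot for the player backpack that snaps and stores one grabbable item.
; Box overlap registers an empty slot as the item's CurrentInventorySlot; the end-overlap clear compares the grabbable component itself to the slot, not that variable.
; StoreItem attaches the item to SnapPoint, saves its original scale, resets relative scale, disables physics, then has the parent BP_PlayerBackpack check whether it is full.
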(event OnComponentBeginOverlap(Box)
  (params (OverlappedComponent :type Primitive%20Component%20Object%20Reference) (OtherActor :type Actor%20Object%20Reference) (OtherComp :type Primitive%20Component%20Object%20Reference) (OtherBodyIndex :type Integer) (bFromSweep :type Boolean) (SweepResult :type Hit%20Result%20Structure%20%28by%20ref%29))
  (bind _returnvalue (Actor|GetComponentbyClass OtherActor "/Game/_Game/Blueprints/BP_GrabbableComponent.BP_GrabbableComponent_C"))
  (Utilities|IsValid _returnvalue
    (:Is%20Valid
      (if (not (Utilities|IsValid (Variables|Default|GetStoredItem)))
        (Variables|/Game/_Game/Blueprints/BP_GrabbableComponent.BP_GrabbableComponent_C|SetCurrentInventorySlot _returnvalue self)))))

(event OnComponentEndOverlap(Box)
  (params (OverlappedComponent :type Primitive%20Component%20Object%20Reference) (OtherActor :type Actor%20Object%20Reference) (OtherComp :type Primitive%20Component%20Object%20Reference) (OtherBodyIndex :type Integer))
  (bind _returnvalue (Actor|GetComponentbyClass OtherActor "/Game/_Game/Blueprints/BP_GrabbableComponent.BP_GrabbableComponent_C"))
  (Utilities|IsValid _returnvalue
    (:Is%20Valid
      (if (== _returnvalue self)
        (Variables|/Game/_Game/Blueprints/BP_GrabbableComponent.BP_GrabbableComponent_C|SetCurrentInventorySlot _returnvalue 0)))))

(fn ConstructionScript)

(fn StoreItem
  (params (Item :type Actor%20Object%20Reference))
  (bind _returnvalue (Actor|GetComponentbyClass Item "/Game/_Game/Blueprints/BP_GrabbableComponent.BP_GrabbableComponent_C"))
  (if (not (Utilities|IsValid (Variables|Default|GetStoredItem)))
    (Transformation|AttachComponentToComponent Item (Variables|Default|GetSnapPoint) "None" "SnapToTarget" "SnapToTarget" "KeepWorld" true)
    (Transformation|SetActorRelativeLocation Item "0, 0, 0" false true)
    (Transformation|SetActorRelativeRotation Item)
    (Utilities|IsValid _returnvalue
      (:Is%20Valid
        (Variables|/Game/_Game/Blueprints/BP_GrabbableComponent.BP_GrabbableComponent_C|SetOriginalScale _returnvalue (Transformation|GetActorScale3D Item))
        (Transformation|SetActorRelativeScale3D Item "1.000000,1.000000,1.000000")
        (Physics|SetSimulatePhysics (Actor|GetComponentbyClass Item "/Script/Engine.StaticMeshComponent") false)
        (Variables|Default|SetStoredItem Item)
        (bind _asbp_player_backpack (Utilities|Casting|CastToBP_PlayerBackpack (Actor|GetAttachParentActor)))
        (Default|CheckInventoryFull _asbp_player_backpack)))))