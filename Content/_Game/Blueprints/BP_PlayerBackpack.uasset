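; BP_PlayerBackpack is a grabbable player backpack that holds items in four inventory slots.
; On BeginPlay it casts four child actors to BP_InventoryComponent and caches them as Slot1 to Slot4, stopping at the first failed cast.
; CheckInventoryFull sets IsInventoryFull according to whether every slot has a valid StoredItem.
; IsGrabbable always returns true.
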(event EventBeginPlay
  (bind _asbp_inventory_component (Utilities|Casting|CastToBP_InventoryComponent (Variables|/Script/Engine.ChildActorComponent|GetChildActor (Variables|Default|GetBP_InventoryComponent1))))
  (Variables|Default|SetSlot1 _asbp_inventory_component)
  (bind _asbp_inventory_component_2 (Utilities|Casting|CastToBP_InventoryComponent (Variables|/Script/Engine.ChildActorComponent|GetChildActor (Variables|Default|GetBP_InventoryComponent2))))
  (Variables|Default|SetSlot2 _asbp_inventory_component_2)
  (bind _asbp_inventory_component_3 (Utilities|Casting|CastToBP_InventoryComponent (Variables|/Script/Engine.ChildActorComponent|GetChildActor (Variables|Default|GetBP_InventoryComponent3))))
  (Variables|Default|SetSlot3 _asbp_inventory_component_3)
  (bind _asbp_inventory_component_4 (Utilities|Casting|CastToBP_InventoryComponent (Variables|/Script/Engine.ChildActorComponent|GetChildActor (Variables|Default|GetBP_InventoryComponent4))))
  (Variables|Default|SetSlot4 _asbp_inventory_component_4))

(fn ConstructionScript)

(fn CheckInventoryFull
  (if (Math|Boolean|ANDBoolean (Utilities|IsValid (Variables|/Game/_Game/Blueprints/BP_InventoryComponent.BP_InventoryComponent_C|GetStoredItem (Variables|Default|GetSlot1))) (Utilities|IsValid (Variables|/Game/_Game/Blueprints/BP_InventoryComponent.BP_InventoryComponent_C|GetStoredItem (Variables|Default|GetSlot2))) (Utilities|IsValid (Variables|/Game/_Game/Blueprints/BP_InventoryComponent.BP_InventoryComponent_C|GetStoredItem (Variables|Default|GetSlot3))) (Utilities|IsValid (Variables|/Game/_Game/Blueprints/BP_InventoryComponent.BP_InventoryComponent_C|GetStoredItem (Variables|Default|GetSlot4))))
    (Variables|Default|SetIsInventoryFull? true)
    (else
      (Variables|Default|SetIsInventoryFull? false))))

(fn IsGrabbable?
  (return true))